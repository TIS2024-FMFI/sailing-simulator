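; Cinematic camera actor that flies in a continuous loop through control points while looking at the world origin.
; On BeginPlay it collects spawn positions from race data table rows named with "cinematiccamera", snaps to the first and disables movement if none exist.
; Each tick it moves in a straight line at constant speed toward the target, switching to the next point, wrapping around, once it gets close.
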(event `self.ReceiveBeginPlay`
  (`self.Load Control Points From Config`)
  ;[1 1 1] Are There Enough Control Points?
  (bind _output_get (set `self.Enabled` (>= (`KismetArrayLibrary.Array_Length` (`self.Control Points`)) 1)))
  (if _output_get
    (`self.Set Location To First Point`)
    (`self.Set Origin And Target` 0)
    (`self.Calculate Direction `)))

(event `self.ReceiveTick`
  (params (DeltaSeconds :type "Float (single-precision)"))
  (if (`self.Enabled`)
    (if (`self.Is Near Target`)
      (`self.Set Origin And Target` (`self.Index Going To`))
      (`self.Calculate Direction `)
      (else
        (`self.K2_AddActorWorldOffset` (* DeltaSeconds (`self.Direction`) (`self.Base Camera Movement Speed`)))
        (`self.Rotate To Center Of World`)))))

(fn `Calculate Direction `
  (set `self.Direction` (`KismetMathLibrary.Normal` (- (`self.Target`) (`self.Origin`)))))

(fn `Is Near Target`
  (returns (`Is Near Target` :type Boolean))
  (return (< (`KismetMathLibrary.Vector_Distance` (`SceneComponent.K2_GetComponentLocation` (`self.DefaultSceneRoot`)) (`self.Target`)) 10.0)))

(fn `Load Control Points From Config`
  (locals (`Row Name` :type Name))
  (bind _outrownames (`DataTableFunctionLibrary.GetDataTableRowNames` "/Game/Map/RaceDataTable.RaceDataTable"))
  (for _array_element _outrownames
    (bind _output_get (set `local.Row Name` _array_element))
    (if (`KismetStringLibrary.Contains` (`KismetStringLibrary.Conv_NameToString` _output_get) "cinematiccamera")
      (bind _returnvalue (`|GetDataTableRow` "/Game/Map/RaceDataTable.RaceDataTable" (`local.Row Name`))
        (:`then`
          (`KismetArrayLibrary.Array_Add` (`self.Control Points`) (`.SpawnPosition_49_747A685D44F6252A8DD5889A6A77C83A` (break `/Game/Map/RaceStructure` _returnvalue)))
          (`/Engine/EditorBlueprintResources/StandardMacros.IncrementInt` (`self.Number Of Control Points`)))))))

(fn `Rotate To Center Of World`
  (`SceneComponent.K2_SetWorldRotation` (`self.Camera`) (`KismetMathLibrary.FindLookAtRotation` (`SceneComponent.K2_GetComponentLocation` (`self.Camera`)) (0.0 0.0 0.0)) false false))

(fn `Set Location To First Point`
  (`self.K2_SetActorLocation` (`|GetArrayItem` (`self.Control Points`))))

(fn `Set Origin And Target`
  (params (`Origin Index` :type Integer))
  (bind _control_points (`self.Control Points`))
  (bind _output (`self.Increment And Modulo` `Origin Index` (`self.Number Of Control Points`)))
  (set `self.Origin` (`|GetArrayItem` _control_points `Origin Index`))
  (set `self.Target` (`|GetArrayItem` _control_points _output))
  (set `self.Index Going To` _output))

(fn `UserConstructionScript`)