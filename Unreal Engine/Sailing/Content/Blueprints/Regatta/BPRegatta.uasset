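; Sailboat actor for a regatta game, with steerable self-centring rudder, adjustable sail tension and click-to-switch boat selection.
; Tick turns the hull, angles the mast to wind read from overlapped grid tiles, and moves by a swept vector updated through an external calculation.
; BeginPlay places extra cameras from the race data table and starts timed render-target snapshot exports, with telemetry encoded in filenames.
; Collision overlaps record buoys reached.
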(event `self.ReceiveTick`
  (params (DeltaSeconds :type "Float (single-precision)"))
  (bind _returnvalue (`GameplayStatics.GetWorldDeltaSeconds`))
  (`|ExecutionSequence`
    (:`then_0`
      ;[1 1 1] Rudder Visual / Control Logic
      (if (or (`self.RudderIsReturning`) (not (`self.Is Possesed`)))
        (`self.Rudder Return Tick` _returnvalue)
        (else
          (`self.Apply Rudder Rotation Direction` _returnvalue)
          (`self.K2_AddActorWorldRotation` (`KismetMathLibrary.MakeRotator` 0.0 0.0 (* _returnvalue (`self.Calculate Turning Tick`) 10.0)))
          (set `self.Movement Vector` (/ (`self.Get Movement Vector`) 1.001)))))
    (:`then_1`
      ;[1 1 1] Sail Tension Logic
      (`self.Sail Tick` (`GameplayStatics.GetWorldDeltaSeconds`)))
    (:`then_2`
      (`/Game/Map/PhysicsEngine.setNewMovementVector` self (`self.Movement Vector`))
      (`self.K2_SetActorLocation` (+ (`self.K2_GetActorLocation`) (* (`self.Movement Vector`) (`GameplayStatics.GetWorldDeltaSeconds`))) true))
    (:`then_3`
      (bind _rotation (`/Game/Map/PhysicsEngine.calculateNewSailAngle` (`self.Current Wind Direction`) (`self.SailTension`) (`SceneComponent.K2_GetComponentRotation` (`self.Hull`))))
      (`SceneComponent.K2_SetWorldRotation` (`self.Mast`) (`KismetMathLibrary.MakeRotator` 0.0 0.0 _rotation) false false))
    (:`then_4`
      (`self.Update Anemometer Rotation`))
    (:`then_5`
      (bind _asplayer_controller (cast `PlayerController` (`self.GetController`)))
      (set `PlayerController.bShowMouseCursor` true _asplayer_controller)
      (bind _asbpregatta (cast `/Game/Blueprints/Regatta/BPRegatta` (`.HitActor` (`GameplayStatics.BreakHitResult` (`PlayerController.GetHitResultUnderCursorForObjects` _asplayer_controller (`|MakeArray` "ObjectTypeQuery2" :!type "EObjectTypeQuery Enum") true)))))
      (bind _asbpregatta_controller (cast `/Game/Blueprints/Regatta/BPRegattaController` (`GameplayStatics.GetPlayerController` 0)))
      (`/Game/Blueprints/Regatta/BPRegattaController.Swap To Boat` _asbpregatta_controller _asbpregatta)
      (bind _assailing_game_instance (cast `/Game/Blueprints/SailingGameInstance` (`GameplayStatics.GetGameInstance`)))
      (bind _minimapwidget (`/Game/Blueprints/SailingGameInstance.Get Minimap Widget` _assailing_game_instance))
      (`/Game/Minimap/MinimapWidget.switchMinimapToBoat` _minimapwidget _asbpregatta))))

(event `self.ReceiveBeginPlay`
  (`KismetSystemLibrary.PrintString` (`KismetStringLibrary.Concat_StrStr` (`KismetSystemLibrary.GetDisplayName` self) " calls BEGIN PLAY"))
  (bind _returnvalue (`|CreateWidget` "/Game/Minimap/MinimapWidget.MinimapWidget_C" (`GameplayStatics.GetPlayerController` 0)))
  (`UserWidget.AddToViewport` _returnvalue 0)
  (`self.Find Data Tile`)
  (`self.Update Wind Data`)
  (`self.Transform Additional Cameras From Config`)
  (`self.SetActorTickEnabled` true)
  (bind _returnvalue_2 (`KismetRenderingLibrary.CreateRenderTarget2D` 256 256 "RTF_RGBA8"))
  (set `SceneCaptureComponent2D.TextureTarget` _returnvalue_2 (`self.Snapshots`))
  (bind _assailing_game_instance (cast `/Game/Blueprints/SailingGameInstance` (`GameplayStatics.GetGameInstance`)))
  (bind _snapfrequen (`/Game/Blueprints/SailingGameInstance.Get snapfrequen` _assailing_game_instance))
  (`KismetSystemLibrary.K2_SetTimer` null "Make Snapshot" (`KismetMathLibrary.Conv_IntToDouble` _snapfrequen) true)
  (bind _returnvalue_3 (`KismetRenderingLibrary.CreateRenderTarget2D` 256 256 "RTF_RGBA8"))
  (set `SceneCaptureComponent2D.TextureTarget` _returnvalue_3 (`self.SceneCaptureComponent2D`)))

(event `self.Grid Tile Detector.OnComponentBeginOverlap`
  (params (OverlappedComponent :type "PrimitiveComponent Object Reference") (OtherActor :type "Actor Object Reference") (OtherComp :type "PrimitiveComponent Object Reference") (OtherBodyIndex :type Integer) (bFromSweep :type Boolean) (SweepResult :type "HitResult Structure (by ref)"))
  (`self.Find Data Tile`)
  (`self.Update Wind Data`))

(event `self.ReceivePossessed`
  (params (NewController :type "Controller Object Reference"))
  ;[1 1 1] Why must god torment me so?
  (set `self.Is Possesed` true))

(event `self.ReceiveUnpossessed`
  (params (OldController :type "Controller Object Reference"))
  ;[1 1 1] Why must god torment me so?
  (set `self.Is Possesed` false))

(event `self.CollisionBox.OnComponentBeginOverlap`
  (params (OverlappedComponent :type "PrimitiveComponent Object Reference") (OtherActor :type "Actor Object Reference") (OtherComp :type "PrimitiveComponent Object Reference") (OtherBodyIndex :type Integer) (bFromSweep :type Boolean) (SweepResult :type "HitResult Structure (by ref)"))
  (bind _asbp_buoy (cast `/Game/Map/BP_Buoy` OtherActor))
  (`BlueprintSetLibrary.Set_Add` (`self.BuoyCounter`) _asbp_buoy))

(event `self.BoatIndicator.OnClicked`
  (params (TouchedComponent :type "PrimitiveComponent Object Reference") (ButtonPressed :type "Key Structure"))
  (bind _asbpregatta_controller (cast `/Game/Blueprints/Regatta/BPRegattaController` (`GameplayStatics.GetPlayerController` 0)))
  (`/Game/Blueprints/Regatta/BPRegattaController.Swap To Boat` _asbpregatta_controller self))

(fn `Activate Chase Camera`
  (`ActorComponent.SetActive` (`self.Chase Camera`) true false))

(fn `Apply Rudder Rotation Direction`
  (params (`Delta Seconds` :type "Float (double-precision)"))
  (bind _rudder (`self.Rudder`))
  (bind _maximumrudderrotation (`self.MaximumRudderRotation`))
  (bind (_relativerotation_roll _relativerotation_pitch _relativerotation_yaw) (`KismetMathLibrary.BreakRotator` (`SceneComponent.RelativeRotation` _rudder)))
  (`SceneComponent.K2_AddRelativeRotation` _rudder (`KismetMathLibrary.MakeRotator` 0.0 0.0 (* `Delta Seconds` (`self.CurrentRudderRotationDelta`))) false false)
  (`SceneComponent.K2_SetRelativeRotation` (`self.Rudder`) (`KismetMathLibrary.MakeRotator` 0.0 0.0 (`KismetMathLibrary.FClamp` _relativerotation_yaw (* _maximumrudderrotation -1.0) _maximumrudderrotation)) false false))

(fn `Calculate Turning Tick`
  (returns (`Delta Angle` :type "Float (double-precision)"))
  (bind (_relativerotation_roll _relativerotation_pitch _relativerotation_yaw) (`KismetMathLibrary.BreakRotator` (`SceneComponent.RelativeRotation` (`self.Rudder`))))
  (return (* (`KismetMathLibrary.SelectFloat` 2.0 0.0 (and (not (`self.RudderIsReturning`)) (> (/ (`self.CurrentRudderRotationDelta`) _relativerotation_yaw) 0.0))) (`KismetMathLibrary.SelectFloat` -1.0 1.0 (>= (`self.CurrentRudderRotationDelta`) 0.0)))))

(fn `Deactivate All Cameras`
  (`ActorComponent.SetActive` (`self.Chase Camera`) false false)
  (`ActorComponent.SetActive` (`self.ExtraCam1`) false false)
  (`ActorComponent.SetActive` (`self.ExtraCam2`) false false)
  (`ActorComponent.SetActive` (`self.ExtraCam3`) false false)
  (`ActorComponent.SetActive` (`self.ExtraCam4`) false false)
  (`ActorComponent.SetActive` (`self.ExtraCam5`) false false)
  (`ActorComponent.SetActive` (`self.ExtraCam6`) false false)
  (`ActorComponent.SetActive` (`self.ExtraCam6`) false false)
  (`ActorComponent.SetActive` (`self.ExtraCam7`) false false)
  (`ActorComponent.SetActive` (`self.ExtraCam8`) false false)
  (`ActorComponent.SetActive` (`self.ExtraCam9`) false false))

(fn `Find Data Tile`
  (for _array_element (`PrimitiveComponent.GetOverlappingActors` (`self.Grid Tile Detector`) null)
    (bind _asbp_tile (cast `/Game/Map/BP_Tile` _array_element))
    (bind _output_get (set `self.Current Tile` _asbp_tile))
    (`KismetSystemLibrary.PrintString` (`KismetStringLibrary.Concat_StrStr` "Current Tile : " (`KismetSystemLibrary.GetDisplayName` _output_get) "(" (`KismetSystemLibrary.GetDisplayName` self) ")"))
    (return)))

(fn `Get Acceleration`
  (returns (Acceleration :type "Float (double-precision)"))
  (return (`self.Acceleration`)))

(fn `Get Camera By Number`
  (params (Index :type Integer))
  (returns (Camera :type "CameraComponent Object Reference"))
  (switch `int` Index
    (:`0`
      (return (`self.ExtraCam1`)))
    (:`1`
      (return (`self.ExtraCam2`)))
    (:`2`
      (return (`self.ExtraCam3`)))
    (:`3`
      (return (`self.ExtraCam4`)))
    (:`4`
      (return (`self.ExtraCam5`)))
    (:`5`
      (return (`self.ExtraCam6`)))
    (:`6`
      (return (`self.ExtraCam7`)))
    (:`7`
      (return (`self.ExtraCam8`)))
    (:`8`
      (return (`self.ExtraCam9`)))))

(fn `Get Hull Area`
  (returns (`Hull Area` :type "Float (double-precision)"))
  (return (`self.Hull Area`)))

(fn `Get Inertia Moment`
  (returns (`Inertia Moment` :type "Float (double-precision)"))
  (return (`self.Moment Of Inertia`)))

(fn `Get Mass`
  (returns (Mass :type "Float (double-precision)"))
  (return (`self.Mass`)))

(fn `Get Max Rudder Angle`
  (returns (`Max Rudder Angle` :type "Float (double-precision)"))
  (return (`self.MaximumRudderRotation`)))

(fn `Get Maximum Lif Coeficient`
  (returns (maxLiftCoeficient :type "Float (double-precision)"))
  (return (`self.MaximumLiftCoeficient`)))

(fn `Get Movement Vector`
  (returns (`Movement Vector` :type "Vector Structure"))
  (return (`self.Movement Vector`)))

(fn `Get Rudder Angle`
  (returns (Rotation :type "Float (double-precision)"))
  (bind (_relativerotation_roll _relativerotation_pitch _relativerotation_yaw) (`KismetMathLibrary.BreakRotator` (`SceneComponent.RelativeRotation` (`self.Rudder`))))
  (return _relativerotation_yaw))

(fn `Get Rudder Angle PHYS`
  (params (`In Radians` :type Boolean))
  (returns (`Rudder Angle` :type "Float (double-precision)"))
  (bind _rotation (`self.Get Rudder Angle`))
  (return (`KismetMathLibrary.SelectFloat` (`KismetMathLibrary.DegreesToRadians` _rotation) _rotation `In Radians`)))

(fn `Get Rudder Area`
  (returns (Area :type "Float (double-precision)"))
  (return (`self.Rudder Area`)))

(fn `Get Rudder Length`
  (returns (Length :type "Float (double-precision)"))
  (return (`self.Rudder Length`)))

(fn `Get Sail Angle`
  (params (`In Radians` :type Boolean))
  (returns (`Sail Angle` :type "Float (double-precision)"))
  (bind _sail_angle (`self.Sail Angle`))
  (return (`KismetMathLibrary.SelectFloat` (`KismetMathLibrary.DegreesToRadians` _sail_angle) _sail_angle `In Radians`)))

(fn `Get Sail Area`
  (returns (`Sail Area` :type "Float (double-precision)"))
  (return (`self.Sail Area`)))

(fn `Get Sail Tension`
  (returns (`Sail Tension` :type "Float (double-precision)"))
  (return (`self.SailTension`)))

(fn `Get Velocity`
  (returns (Velocity :type "Float (double-precision)"))
  (return (`self.Velocity`)))

(fn `Make Snapshot`
  (bind (_returnvalue_x _returnvalue_y _returnvalue_z) (`KismetMathLibrary.BreakVector` (`self.K2_GetActorLocation`)))
  (bind (_returnvalue_x_2 _returnvalue_y_2 _returnvalue_z_2) (`KismetMathLibrary.BreakVector` (`self.GetActorForwardVector`)))
  (bind (_current_wind_direction_x _current_wind_direction_y _current_wind_direction_z) (`KismetMathLibrary.BreakVector` (`self.Current Wind Direction`)))
  (bind _current_tile (`self.Current Tile`))
  (bind _returnvalue (`KismetMathLibrary.FFloor64` (`KismetSystemLibrary.GetGameTimeInSeconds`)))
  (bind (_waterdirection_x _waterdirection_y _waterdirection_z) (`KismetMathLibrary.BreakVector` (`/Game/Map/BP_Tile.WaterDirection` _current_tile)))
  (bind _returnvalue_2 (mod _returnvalue 3600))
  (`KismetRenderingLibrary.ExportRenderTarget` (`SceneCaptureComponent2D.TextureTarget` (`self.Snapshots`)) (`KismetStringLibrary.Concat_StrStr` (`KismetSystemLibrary.GetProjectSavedDirectory`) "Snapshots/" (`KismetSystemLibrary.GetDisplayName` self)) (`KismetTextLibrary.Conv_TextToString` (`|FormatText` "{Regatta}_{Counter}_{Time}_{WindSpeed}_{WindDirection}_{WaterSpeed}_{WaterDirection}_{SailTension}_{SailRotation}_{RudderRotation}_{coordinates}_{RegattaDirection}.png" (`KismetSystemLibrary.GetDisplayName` self) (`self.Snapshot Counter`) (`|FormatText` "({Hours}-{Minutes}-{Seconds})" (/ _returnvalue 3600) (/ _returnvalue_2 60) (mod _returnvalue_2 60)) (`self.Current Wind Speed`) (`|FormatText` "(X{X},Y{Y},Z{Z})" (/ (`KismetMathLibrary.Conv_IntToDouble` (`KismetMathLibrary.Round` (* _current_wind_direction_x 100.0))) 100.0) (/ (`KismetMathLibrary.Conv_IntToDouble` (`KismetMathLibrary.Round` (* _current_wind_direction_y 100.0))) 100.0) (/ (`KismetMathLibrary.Conv_IntToDouble` (`KismetMathLibrary.Round` (* _current_wind_direction_z 100.0))) 100.0)) (`/Game/Map/BP_Tile.WaterSpeed` _current_tile) (`|FormatText` "(X{X},Y{Y},Z{Z})" (/ (`KismetMathLibrary.Conv_IntToDouble` (`KismetMathLibrary.Round` (* _waterdirection_x 100.0))) 100.0) (/ (`KismetMathLibrary.Conv_IntToDouble` (`KismetMathLibrary.Round` (* _waterdirection_y 100.0))) 100.0) (/ (`KismetMathLibrary.Conv_IntToDouble` (`KismetMathLibrary.Round` (* _waterdirection_z 100.0))) 100.0)) (`self.SailTension`) (`self.Sail Angle`) (`self.Get Rudder Angle`) (`|FormatText` "(X{X},Y{Y},Z{Z})" (/ (`KismetMathLibrary.Conv_IntToDouble` (`KismetMathLibrary.Round` (* _returnvalue_x 100.0))) 100.0) (/ (`KismetMathLibrary.Conv_IntToDouble` (`KismetMathLibrary.Round` (* _returnvalue_y 100.0))) 100.0) (/ (`KismetMathLibrary.Conv_IntToDouble` (`KismetMathLibrary.Round` (* _returnvalue_z 100.0))) 100.0)) (`|FormatText` "(X{X},Y{Y},Z{Z})" (/ (`KismetMathLibrary.Conv_IntToDouble` (`KismetMathLibrary.Round` (* _returnvalue_x_2 100.0))) 100.0) (/ (`KismetMathLibrary.Conv_IntToDouble` (`KismetMathLibrary.Round` (* _returnvalue_y_2 100.0))) 100.0) (/ (`KismetMathLibrary.Conv_IntToDouble` (`KismetMathLibrary.Round` (* _returnvalue_z_2 100.0))) 100.0)))))
  (set `self.Snapshot Counter` (+ (`self.Snapshot Counter`) 1)))

(fn `Movement Tick`
  (`KismetSystemLibrary.PrintString` "Movement = TODO"))

(fn `Rudder Return Tick`
  (params (`Delta Seconds` :type "Float (double-precision)"))
  (bind _rudder (`self.Rudder`))
  (bind (_relativerotation_roll _relativerotation_pitch _relativerotation_yaw) (`KismetMathLibrary.BreakRotator` (`SceneComponent.RelativeRotation` (`self.Rudder`))))
  (bind (_relativerotation_roll_2 _relativerotation_pitch_2 _relativerotation_yaw_2) (`KismetMathLibrary.BreakRotator` (`SceneComponent.RelativeRotation` _rudder)))
  (`SceneComponent.K2_AddRelativeRotation` _rudder (`KismetMathLibrary.MakeRotator` 0.0 0.0 (* (`KismetMathLibrary.SelectFloat` -1.0 1.0 (>= _relativerotation_yaw 0.0)) (`self.RudderRotationConstant`) `Delta Seconds`)) false false)
  (if (<= (`KismetMathLibrary.Abs` _relativerotation_yaw_2) 3.0)
    (`SceneComponent.K2_SetRelativeRotation` :`self` (`self.Rudder`))
    (set `self.RudderIsReturning` false)))

(fn `Sail Tick`
  (params (`Delta Seconds` :type "Float (double-precision)"))
  (set `self.SailTension` (`KismetMathLibrary.FClamp` (+ (* `Delta Seconds` (`self.ConstantSailTensionDelta`) (`self.SailAxisValue`)) (`self.SailTension`)) 0.0 100.0)))

(fn `Set New Movement Vector`
  (params (`New Movement Vector` :type "Vector Structure"))
  (set `self.Movement Vector` `New Movement Vector`))

(fn `Set Rudder Is Returning`
  (params (`Is Returning` :type Boolean))
  (set `self.RudderIsReturning` `Is Returning`))

(fn `Set Rudder Rotation Direction`
  (params (Input :type "Float (double-precision)"))
  (bind _output_get (set `self.CurrentRudderRotationDelta` (* Input (`self.RudderRotationConstant`)))))

(fn `Set Sail Axis Value`
  (params (`New Sail Axis Value` :type "Float (double-precision)"))
  (set `self.SailAxisValue` `New Sail Axis Value`))

(fn `Transform Additional Cameras From Config`
  (locals (`Row Name` :type Name) (`Camera Index` :type Integer))
  (bind _returnvalue (`KismetStringLibrary.Conv_NameToString` (`local.Row Name`)))
  (bind _outrownames (`DataTableFunctionLibrary.GetDataTableRowNames` "/Game/Map/RaceDataTable.RaceDataTable"))
  (for _array_element _outrownames
    (bind _output_get (set `local.Row Name` _array_element))
    (if (`KismetStringLibrary.Contains` (`KismetStringLibrary.Conv_NameToString` _output_get) "usercamera")
      (set `local.Camera Index` (- (`KismetStringLibrary.Conv_StringToInt` (`KismetStringLibrary.RightChop` _returnvalue (- (`KismetStringLibrary.Len` _returnvalue) 1))) 1))
      (bind _returnvalue_2 (`|GetDataTableRow` "/Game/Map/RaceDataTable.RaceDataTable" (`local.Row Name`))
        (:`then`
          (bind (_gridrow _gridcolumn _winddirection _windspeed _waterdirection _waterspeed _depth _spawnindex _spawnposition _angle) (break `/Game/Map/RaceStructure` _returnvalue_2))
          (`SceneComponent.K2_SetRelativeLocationAndRotation` (`self.Get Camera By Number` (`local.Camera Index`)) (* _spawnposition 200.0) (`KismetMathLibrary.MakeRotator` (.x _angle) (.y _angle) (.z _angle)) false false))))))

(fn `Update Anemometer Rotation`
  (`SceneComponent.K2_SetWorldRotation` (`self.Anemometer`) (`KismetMathLibrary.MakeRotFromX` (`self.Current Wind Direction`)) false false))

(fn `Update Wind Data`
  (bind _current_tile (`self.Current Tile`))
  (set `self.Current Wind Direction` (`/Game/Map/BP_Tile.WindDirection` _current_tile))
  (set `self.Current Wind Speed` (`KismetMathLibrary.Conv_IntToDouble` (`/Game/Map/BP_Tile.WindSpeed` _current_tile))))

(fn `UserConstructionScript`)