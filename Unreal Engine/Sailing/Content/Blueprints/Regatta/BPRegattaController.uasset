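; Player controller for the regatta boat, handling rudder and sail input, camera switching and the HUD.
; BeginPlay creates the RegattaUI, caches the possessed BPRegatta and enables extra cameras from "usercamera" data table rows.
; Inputs drive the cached boat and sail tension bar, while Tick refreshes the rudder slider.
; View changes cover chase, numbered, cinematic and orthogonal cameras, and SwapToBoat possesses another boat in chase view.
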(event `Swap To Boat`
  (params (`New Boat` :type "/Game/Blueprints/Regatta/BPRegatta Object Reference"))
  (bind _cast_regatta (`self.Cast Regatta`))
  (`self.UnPossess`)
  (bind _output_get (set `self.Cast Regatta` `New Boat`))
  (`self.Possess` _output_get)
  (`/Game/Blueprints/Regatta/BPRegatta.Deactivate All Cameras` _cast_regatta)
  (`/Game/Blueprints/Regatta/BPRegatta.Activate Chase Camera` _cast_regatta)
  (`self.SetViewTargetWithBlend` (`self.Cast Regatta`) 2.0))

(event `self.ReceiveBeginPlay`
  ;[1 1 1] Create And Place HUD
  (bind _returnvalue (`|CreateWidget` "/Game/Blueprints/Regatta/RegattaUI.RegattaUI_C"))
  (`UserWidget.AddToViewport` _returnvalue 0)
  (set `self.UI Widget` _returnvalue)
  ;[1 1 1] Save Cast Pointer (to avoid redundant future casts cos its expensive)
  (bind _asbpregatta (cast `/Game/Blueprints/Regatta/BPRegatta` (`self.K2_GetPawn`)))
  (set `self.Cast Regatta` _asbpregatta)
  (`self.Enable Cameras From Config`)
  (set `self.bShowMouseCursor` true)
  (`WidgetBlueprintLibrary.SetInputMode_GameAndUIEx` self null))

(event `InputAxis|Rudder Axis`
  (params (AxisValue :type "Float (single-precision)"))
  (bind _cast_regatta (`self.Cast Regatta`))
  ;[1 1 1] Rudder Controls
  (if (!= AxisValue 0.0)
    (`/Game/Blueprints/Regatta/BPRegatta.Set Rudder Rotation Direction` _cast_regatta (`self.GetInputAxisValue`))
    (`/Game/Blueprints/Regatta/BPRegatta.Set Rudder Is Returning` _cast_regatta false)
    (else
      (`/Game/Blueprints/Regatta/BPRegatta.Set Rudder Is Returning` _cast_regatta true)
      (`/Game/Blueprints/Regatta/BPRegatta.Set Rudder Rotation Direction` _cast_regatta 0.0))))

(event `InputAxis|Sail Tension Axis`
  (params (AxisValue :type "Float (single-precision)"))
  (`/Game/Blueprints/Regatta/BPRegatta.Set Sail Axis Value` (`self.Cast Regatta`) AxisValue)
  (`/Game/Blueprints/Regatta/RegattaUI.Update Sail Tension Bar` (`self.UI Widget`) (`/Game/Blueprints/Regatta/BPRegatta.Get Sail Tension` (`self.Cast Regatta`))))

(event `self.ReceiveTick`
  (params (DeltaSeconds :type "Float (single-precision)"))
  (bind _cast_regatta (`self.Cast Regatta`))
  (bind _ui_widget (`self.UI Widget`))
  (`/Game/Blueprints/Regatta/RegattaUI.Set Slider Value` _ui_widget (`/Game/Blueprints/Regatta/RegattaUI.Rudder Angle To Turning Slider Pct` _ui_widget (`/Game/Blueprints/Regatta/BPRegatta.Get Max Rudder Angle` _cast_regatta) (`/Game/Blueprints/Regatta/BPRegatta.Get Rudder Angle` _cast_regatta))))

(event `InputAction|Extra Camera Swapping`
  (params (Key :type "Key Structure"))
  (bind _returnvalue (`self.Number Key X to Int(X) - 1` Key))
  (bind _cast_regatta (`self.Cast Regatta`))
  (:`Pressed`
    (if (`|GetArrayItem` (`self.Camera Active Staus`) _returnvalue)
      (`/Game/Blueprints/Regatta/BPRegatta.Deactivate All Cameras` _cast_regatta)
      (`ActorComponent.SetActive` (`/Game/Blueprints/Regatta/BPRegatta.Get Camera By Number` _cast_regatta _returnvalue) true true)
      (`self.SetViewTargetWithBlend` (`self.Cast Regatta`) 2.0))))

(event `InputAction|Swap To Chase Camera`
  (params (Key :type "Key Structure"))
  (bind _cast_regatta (`self.Cast Regatta`))
  (:`Pressed`
    (`/Game/Blueprints/Regatta/BPRegatta.Deactivate All Cameras` _cast_regatta)
    (`/Game/Blueprints/Regatta/BPRegatta.Activate Chase Camera` _cast_regatta)
    (`self.SetViewTargetWithBlend` (`self.Cast Regatta`) 2.0)))

(event `SwitchToOrthogonalView`
  (bind _outactors (`GameplayStatics.GetAllActorsOfClass` "/Script/Engine.CameraActor"))
  (for _array_element _outactors
    (bind _ascamera_actor (cast `CameraActor` _array_element))
    (if (`KismetStringLibrary.EqualEqual_StrStr` (`KismetSystemLibrary.GetDisplayName` _ascamera_actor) "OrthogonalCamera")
      (set `self.OrthogonalCamera` _ascamera_actor)
      (`self.SetViewTargetWithBlend` (`self.OrthogonalCamera`)))))

(event `InputAction|Swap To Cinematic Camera`
  (params (Key :type "Key Structure"))
  (:`Pressed`
    (`self.Swap To Cinematic`)))

(fn `Enable Cameras From Config`
  (locals (`Row Name` :type String) (`Extra Cameras Enabled` :type Integer))
  (bind _row_name (`local.Row Name`))
  (bind _outrownames (`DataTableFunctionLibrary.GetDataTableRowNames` "/Game/Map/tutorial_tabel.tutorial_tabel"))
  (for _array_element _outrownames
    (bind _output_get (set `local.Row Name` (`KismetStringLibrary.Conv_NameToString` _array_element)))
    (if (`KismetStringLibrary.Contains` _output_get "usercamera")
      (`KismetArrayLibrary.Array_Set` (`self.Camera Active Staus`) (- (`KismetStringLibrary.Conv_StringToInt` (`KismetStringLibrary.RightChop` _row_name (- (`KismetStringLibrary.Len` _row_name) 1))) 1) true)
      (`/Engine/EditorBlueprintResources/StandardMacros.IncrementInt` (`local.Extra Cameras Enabled`))))
  (`KismetSystemLibrary.PrintString` (`KismetStringLibrary.Concat_StrStr` "Enabled " (`KismetStringLibrary.Conv_IntToString` (`local.Extra Cameras Enabled`)) " additional cameras.")))

(fn `Swap To Cinematic`
  (bind _cast_regatta (`self.Cast Regatta`))
  (bind _output_get (set `self.Is In Cinematic Camera` (not (`self.Is In Cinematic Camera`))))
  (if _output_get
    (bind _outactors (`GameplayStatics.GetAllActorsOfClass` "/Game/Blueprints/CinematicCamera/CinematicCameraActor.CinematicCameraActor_C"))
    (`self.SetViewTargetWithBlend` (`|GetArrayItem` _outactors))
    (else
      (`/Game/Blueprints/Regatta/BPRegatta.Deactivate All Cameras` _cast_regatta)
      (`/Game/Blueprints/Regatta/BPRegatta.Activate Chase Camera` _cast_regatta)
      (`self.SetViewTargetWithBlend` (`self.Cast Regatta`) 2.0))))

(fn `UserConstructionScript`)