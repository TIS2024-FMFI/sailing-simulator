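; SailingGameInstance is the sailing game's game instance, holding setup values for boat count, buoy count and spawn location.
; Each value has a plain getter and setter pair that reads or writes the variable directly, with no validation or other logic.
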(fn `Get Boat Count`
  (returns (Boats :type Integer))
  (return (`self.BoatCount`)))

(fn `Get BuoyCount`
  (returns (Bouys :type Integer))
  (return (`self.BuoyCount`)))

(fn `Get SpawnLocation`
  (returns (`New SpawnLocation` :type "Transform Structure"))
  (return (`self.SpawnLocation`)))

(fn `Set Boat Count`
  (params (`New Boat Count` :type Integer))
  (set `self.BoatCount` `New Boat Count`))

(fn `Set Bouy Count`
  (params (`New BouyCount` :type Integer))
  (set `self.BuoyCount` `New BouyCount`))

(fn `Set SpawnLocation`
  (params (`New SpawnLocation` :type "Transform Structure"))
  (set `self.SpawnLocation` `New SpawnLocation`))