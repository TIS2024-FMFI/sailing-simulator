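; BP_Tile is one cell of a sailing map grid, set up through its Initialize function rather than BeginPlay.
; With a valid owner, it attaches to that actor, scales its Tile component by TileWidth and offsets itself by Column and Row using the component's bounds.
; SpawnIndex then selects an optional spawn above it: a start point saved as SailingGameInstance's spawn location, or a buoy that increments its buoy count.
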(fn `Initialize`
  (bind _returnvalue (`self.GetOwner`))
  (bind _returnvalue_2 (`GameplayStatics.GetGameInstance`))
  (bind _returnvalue_3 (`KismetMathLibrary.Conv_IntToDouble` (`self.TileWidth`)))
  (bind _returnvalue_4 (`KismetMathLibrary.MakeVector` (.x (`self.K2_GetActorLocation`)) (.y (`self.K2_GetActorLocation`)) (+ (.z (`self.K2_GetActorLocation`)) 30.0)))
  (bind _returnvalue_5 (`KismetMathLibrary.Conv_VectorToTransform` _returnvalue_4))
  (`/Engine/EditorBlueprintResources/StandardMacros.IsValid` _returnvalue
    (:`Is Valid`
      (`self.K2_AttachToActor` _returnvalue "None" "SnapToTarget" "SnapToTarget" "KeepRelative" false)
      (`SceneComponent.SetRelativeScale3D` (`self.Tile`) (`KismetMathLibrary.MakeVector` _returnvalue_3 _returnvalue_3 0.5))
      (`self.K2_SetActorRelativeLocation` (`KismetMathLibrary.MakeVector` (* (* (.x (`.BoxExtent` (`KismetSystemLibrary.GetComponentBounds` (`self.Tile`)))) 2.0) (`self.Column`)) (* (* (.y (`.BoxExtent` (`KismetSystemLibrary.GetComponentBounds` (`self.Tile`)))) 2.0) (`self.Row`))))
      (switch `int` (`self.SpawnIndex`)
        (:`1`
          (`|SpawnActorFromClass` "/Game/Map/BP_Start.BP_Start_C" _returnvalue_5 "AlwaysSpawn" "MultiplyWithRoot" null null)
          (bind _assailing_game_instance (cast `/Game/Blueprints/SailingGameInstance` _returnvalue_2))
          (`/Game/Blueprints/SailingGameInstance.Set SpawnLocation` _assailing_game_instance _returnvalue_5))
        (:`2`
          (`|SpawnActorFromClass` "/Game/Map/BP_Buoy.BP_Buoy_C" (`KismetMathLibrary.Conv_VectorToTransform` _returnvalue_4) "AlwaysSpawn" "MultiplyWithRoot" null (`self.ActorRotation`) null)
          (bind _assailing_game_instance_2 (cast `/Game/Blueprints/SailingGameInstance` _returnvalue_2))
          (`/Game/Blueprints/SailingGameInstance.Set Bouy Count` _assailing_game_instance_2 (+ (`/Game/Blueprints/SailingGameInstance.Get BuoyCount` _assailing_game_instance_2) 1)))))))

(fn `UserConstructionScript`)